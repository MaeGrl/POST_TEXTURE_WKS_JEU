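; BP_vanne is a player-driven vehicle pawn with a checkpoint-style respawn.
; AVANCER, RECULER and TOURNER axis inputs feed throttle, brake and steering on the vehicle movement component.
; It saves its starting transform, which SetRespawnPosition can replace, and Respawn teleports back there, optionally zeroing velocity with a brief handbrake.
; The stuck action only prints a debug message, while disconnected nodes hold an unused lift-and-level recovery.
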(event `self.ReceiveBeginPlay`
  (`parent.ReceiveBeginPlay`)
  (`self.SetRespawnPosition` (`self.GetTransform`)))

(event `Respawn`
  (params (KeepVelocity :type Boolean))
  (`self.K2_SetActorTransform` (`self.LastRespawnPosition`) false true)
  (if (not KeepVelocity)
    (`ChaosVehicleMovementComponent.SetHandbrakeInput` (`self.VehicleMovementComponent`) true)
    (`PrimitiveComponent.SetAllPhysicsLinearVelocity` (`self.Mesh`) (0.0 0.0 0.0) false)
    (`KismetSystemLibrary.Delay` 0.2)
    (`ChaosVehicleMovementComponent.SetHandbrakeInput` (`self.VehicleMovementComponent`) false)))

(event `EnhancedInput|/Game/GD_Template/Blueprints/stuck`
  (params (ActionValue :type Boolean) (ElapsedSeconds :type "Float (double-precision)") (TriggeredSeconds :type "Float (double-precision)") (InputAction :type "InputAction Object Reference" :default "/Game/GD_Template/Blueprints/stuck.stuck"))
  (:`Triggered`
    (`KismetSystemLibrary.PrintString` "Hello")))

(event `InputAxis|STUCK`
  (params (AxisValue :type "Float (single-precision)")))

(event `InputAxis|AVANCER`
  (params (AxisValue :type "Float (single-precision)"))
  (`ChaosVehicleMovementComponent.SetThrottleInput` (`self.VehicleMovementComponent`) AxisValue))

(event `InputAxis|TOURNER`
  (params (AxisValue :type "Float (single-precision)"))
  (`ChaosVehicleMovementComponent.SetSteeringInput` (`self.VehicleMovementComponent`) AxisValue))

(event `InputAxis|RECULER`
  (params (AxisValue :type "Float (single-precision)"))
  (`ChaosVehicleMovementComponent.SetBrakeInput` (`self.VehicleMovementComponent`) AxisValue))

(fn `SetRespawnPosition`
  (params (RespawnPos :type "Transform Structure"))
  (set `self.LastRespawnPosition` RespawnPos))

(fn `UserConstructionScript`
  (`parent.UserConstructionScript`))