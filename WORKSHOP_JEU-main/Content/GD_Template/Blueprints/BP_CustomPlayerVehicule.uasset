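; BP_CustomPlayerVehicule is a player vehicle Blueprint that adds throttle input and a respawn system.
; It saves its starting transform on BeginPlay, and SetRespawnPosition can replace that stored point.
; Respawn teleports the vehicle there; unless velocity is kept, it zeroes the mesh's linear velocity and briefly holds the handbrake.
; IA_Throttle Triggered and Canceled events pass their value straight to the vehicle movement component.
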(event `self.ReceiveBeginPlay`
  (`parent.ReceiveBeginPlay`)
  (`self.SetRespawnPosition` (`self.GetTransform`)))

(event `Respawn`
  (params (KeepVelocity :type Boolean))
  (`self.K2_SetActorTransform` (`self.LastRespawnPosition`) false true)
  (if (not KeepVelocity)
    (`ChaosVehicleMovementComponent.SetHandbrakeInput` (`self.VehicleMovementComponent`) true)
    (`PrimitiveComponent.SetAllPhysicsLinearVelocity` (`self.Mesh`) (0.0 0.0 0.0) false)
    (`KismetSystemLibrary.Delay` 0.2)
    (`ChaosVehicleMovementComponent.SetHandbrakeInput` (`self.VehicleMovementComponent`) false)))

(event `EnhancedInput|/Game/GD_Template/VehicleTemplate/Input/Actions/IA_Throttle`
  (params (ActionValue :type "Float (double-precision)") (ElapsedSeconds :type "Float (double-precision)") (TriggeredSeconds :type "Float (double-precision)") (InputAction :type "InputAction Object Reference" :default "/Game/GD_Template/VehicleTemplate/Input/Actions/IA_Throttle.IA_Throttle"))
  (:`Triggered`
    (`ChaosVehicleMovementComponent.SetThrottleInput` (`self.VehicleMovementComponent`) ActionValue :!label _label))
  (:`Canceled`
    (goto _label)))

(fn `SetRespawnPosition`
  (params (RespawnPos :type "Transform Structure"))
  (set `self.LastRespawnPosition` RespawnPos))

(fn `UserConstructionScript`
  (`parent.UserConstructionScript`))